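; Ghost wall preview actor for build mode, showing where a wall will be placed and whether the spot is valid.
; ConstructWall briefly spawns the wall class to copy its mesh and proxy, which GetConstructionStruct returns with the ghost's transform.
; A gated Tick snaps the cursor position to the grid, then checks overlaps and slope.
; Five line traces measure slope, a box trace sets height, and failures swap in an error material.
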(event `OnSpawn`
  (params (DisplayMesh :type "StaticMesh Object Reference") (WallClass :type "/Game/RollOut/Blueprints/Walls/MasterBPs/WallMasterBP Class Reference") (ConstrcutionProxy :type "/Game/RollOut/Blueprints/Construction/ConstructionProxyBP Class Reference"))
  ;[1 1 1] OnSpawn
  (if (not (`self.isActive`))
    (set `self.WallClass` WallClass)
    (set `self.ConstructionProxy` ConstrcutionProxy)
    (set `self.DisplayMesh` DisplayMesh)
    (set `self.isActive` true)
    (set `/Game/RollOut/Blueprints/RollOutGamePlay/RollOutCameraPawnController.BuildModeActive` true (`self.ControllerRef`))
    (`StaticMeshComponent.SetStaticMesh` (`self.GhostWallMesh`) (`self.DisplayMesh`))
    (`self.OpenTickGate`)
    (`self.SetMaterial` (not (`self.IsOverlapping`)))
    (set `self.Extent` (`.BoxExtent` (`KismetSystemLibrary.GetComponentBounds` (`self.GhostWallMesh`))))))

(event `KillGhost`
  ;[1 1 1] KillSpawn
  (set `self.WallClass` null)
  (set `self.ConstructionProxy` null)
  (`self.CloseTickGate`)
  (set `self.DisplayMesh` null)
  (set `self.isActive` false)
  (set `/Game/RollOut/Blueprints/RollOutGamePlay/RollOutCameraPawnController.BuildModeActive` false (`self.ControllerRef`))
  (`StaticMeshComponent.SetStaticMesh` (`self.GhostWallMesh`) (`self.DisplayMesh`)))

(event `RotateRight`
  ;[1 1 1] RotateWall
  (`self.K2_SetActorRotation` (`KismetMathLibrary.MakeRotator` (.roll (`self.K2_GetActorRotation`)) (.pitch (`self.K2_GetActorRotation`)) (- (.yaw (`self.K2_GetActorRotation`)) (`self.BuildingRotationRate`)))))

(event `RotateLeft`
  ;[1 1 1] RotateWall
  (`self.K2_SetActorRotation` (`KismetMathLibrary.MakeRotator` (.roll (`self.K2_GetActorRotation`)) (.pitch (`self.K2_GetActorRotation`)) (+ (.yaw (`self.K2_GetActorRotation`)) (`self.BuildingRotationRate`)))))

(event `/Game/RollOut/Blueprints/HUD/IF_RollOutHUD.ConstructWall`
  (params (MainWall :type "/Game/RollOut/Blueprints/Walls/MasterBPs/WallMasterBP Class Reference"))
  ;[1 1 1] WallConstruction
  (bind _returnvalue (`|SpawnActorFromClass` MainWall (`KismetMathLibrary.MakeTransform` (0.0 0.0 0.0)) "Undefined" "OverrideRootScale" null (`self.ControllerRef`)))
  (`|ExecutionSequence`
    (:`then_0`
      (bind _aswall_master_bp (castclass `/Game/RollOut/Blueprints/Walls/MasterBPs/WallMasterBP` MainWall))
      (`self.KillGhost` self)
      (`self.OnSpawn` self (`/Game/RollOut/Blueprints/Walls/MasterBPs/WallMasterBP.DisplayMesh` _returnvalue) _aswall_master_bp (`/Game/RollOut/Blueprints/Walls/MasterBPs/WallMasterBP.ConstructionProxy` _returnvalue)))
    (:`then_1`
      (`self.K2_DestroyActor` _returnvalue))))

(event `self.ReceiveTick`
  (params (DeltaSeconds :type "Float (single-precision)"))
  ;[1 1 1] TickEvent
  (`/Engine/EditorBlueprintResources/StandardMacros.Gate` true :!label _label
    (:`Exit`
      (`self.K2_SetActorLocation` self (`self.SetGridSnapVector`) false false)
      (if (`self.CheckOverlap`)
        (`self.SetMaterial` true)
        (else
          (bind _badlocation (`self.CalculateSlope`))
          (`self.SetMaterial` _badlocation))))))

(event `InputTouch`
  (params (Location :type "Vector Structure") (FingerIndex :type "ETouchIndex Enum"))
  (bind _returnvalue (`|EnumEquality` FingerIndex "Touch1"))
  ;[1 1 1] TickEvent
  (:`Pressed`
    (if _returnvalue
      (goto _label :!via `Open`)))
  (:`Released`
    (if (not _returnvalue)
      (goto _label :!via `Close`))))

(event `OpenTickGate`
  ;[1 1 1] TickEvent
  (goto _label :!via `Open`))

(event `CloseTickGate`
  ;[1 1 1] TickEvent
  (goto _label :!via `Close`))

(event `SetMaterial`
  (params (IsError :type Boolean))
  (bind _ghostwallmesh (`self.GhostWallMesh`))
  ;[1 1 1] ErrorMaterialGhost
  (if (not (== IsError (`self.IsOverlapping`)))
    (bind _output_get (set `self.IsOverlapping` IsError))
    (if _output_get
      (`PrimitiveComponent.SetMaterial` _ghostwallmesh 0 "/Game/RollOut/Materials/GhostErrorM_Inst.GhostErrorM_Inst")
      (else
        (`PrimitiveComponent.SetMaterial` _ghostwallmesh 0 "/Game/RollOut/Materials/GhostM_Inst.GhostM_Inst")))))

(fn `CalculateSlope`
  (returns (BadLocation :type Boolean))
  (locals (Differences :type "Array of Float (double-precision)") (MaxDifferences :type "Float (double-precision)" :default 20.0))
  (bind (_actor_location _forwardvector _rightvector) (`self.GetVectors`))
  (bind (_actor_location_2 _forwardvector_2 _rightvector_2) (`self.GetVectors`))
  (bind (_actor_location_3 _forwardvector_3 _rightvector_3) (`self.GetVectors`))
  (bind _actor_location_4 (`self.GetVectors`))
  (bind _actor_location_5 (`self.GetVectors`))
  (bind (_actor_location_6 _forwardvector_4 _rightvector_4) (`self.GetVectors`))
  (bind _differences (`local.Differences`))
  (bind (_extent_x _extent_y) (`KismetMathLibrary.BreakVector` (`self.Extent`)))
  (bind _maxdifferences (`local.MaxDifferences`))
  (bind (_indexofminvalue _minvalue) (`KismetMathLibrary.MinOfFloatArray` _differences))
  (bind (_indexofmaxvalue _maxvalue) (`KismetMathLibrary.MaxOfFloatArray` _differences))
  (`|ExecutionSequence`
    (:`then_0`
      (`|ExecutionSequence`
        (:`then_0`
          (bind _difference (`self.SlopeTrace` (+ _actor_location_6 (* (+ _forwardvector_4 _rightvector_4) (`self.Extent`)))))
          (`KismetArrayLibrary.Array_Add` (`local.Differences`) _difference))
        (:`then_1`
          (bind _difference_2 (`self.SlopeTrace` (+ _actor_location (* (+ (* _forwardvector -1.0) _rightvector) (`self.Extent`)))))
          (`KismetArrayLibrary.Array_Add` (`local.Differences`) _difference_2))
        (:`then_2`
          (bind _difference_3 (`self.SlopeTrace` (+ _actor_location_2 (* (+ _forwardvector_2 (* _rightvector_2 -1.0)) (`self.Extent`)))))
          (`KismetArrayLibrary.Array_Add` (`local.Differences`) _difference_3))
        (:`then_3`
          (bind _difference_4 (`self.SlopeTrace` (+ _actor_location_3 (* (+ (* _forwardvector_3 -1.0) (* _rightvector_3 -1.0)) (`self.Extent`)))))
          (`KismetArrayLibrary.Array_Add` (`local.Differences`) _difference_4))
        (:`then_4`
          (bind _difference_5 (`self.SlopeTrace` (`self.GetVectors`)))
          (`KismetArrayLibrary.Array_Add` (`local.Differences`) _difference_5))))
    (:`then_1`
      (if (and (> _indexofminvalue -1) (> _indexofmaxvalue -1))
        (bind (_outhit _returnvalue) (`KismetSystemLibrary.BoxTraceSingle` (+ _actor_location_4 (0.0 0.0 1000.0)) (- _actor_location_4 (0.0 0.0 1000.0)) (`KismetMathLibrary.MakeVector` _extent_x _extent_y 1.0) (struct) "TraceTypeQuery3"))
        (if _returnvalue
          (`self.K2_SetActorLocation` (`KismetMathLibrary.MakeVector` (.x _actor_location_5) (.y _actor_location_5) (.z (`.ImpactPoint` (`GameplayStatics.BreakHitResult` _outhit))))))))
    (:`then_2`
      (return (or (> (`KismetMathLibrary.Abs` _minvalue) _maxdifferences) (> (`KismetMathLibrary.Abs` _maxvalue) _maxdifferences))))))

(fn `CheckOverlap`
  (returns (Overlapping :type Boolean))
  (return (> (`KismetArrayLibrary.Array_Length` (`self.GetOverlappingActors` "/Script/Engine.Actor")) 0)))

(fn `GetConstructionStruct`
  (returns (ConstructionStruct :type "/Game/RollOut/Structs/ConstructionStruct Structure"))
  ;[1 1 1] ConstructionStruct
  (return (make `/Game/RollOut/Structs/ConstructionStruct` (`self.WallClass`) (`self.ConstructionProxy`) (`KismetMathLibrary.MakeTransform` (`self.K2_GetActorLocation`) (`self.K2_GetActorRotation`)) (`self.DisplayMesh`))))

(fn `GetIsOverlapping`
  (returns (IsOverlapping :type Boolean))
  (return (`self.IsOverlapping`)))

(fn `GetVectors`
  (returns (`Actor Location` :type "Vector Structure") (ForwardVector :type "Vector Structure") (RightVector :type "Vector Structure"))
  (bind _returnvalue (`self.K2_GetActorRotation`))
  (return (`self.K2_GetActorLocation`) (`KismetMathLibrary.GetForwardVector` _returnvalue) (`KismetMathLibrary.GetRightVector` _returnvalue)))

(fn `SetCursorPosition`
  (params (CursorLocation :type "Vector Structure"))
  (set `self.CursorWorldPosition` CursorLocation)
  (return))

(fn `SetGridSnapVector`
  (returns (GridSnap :type "Vector Structure"))
  (bind (_cursorworldposition_x _cursorworldposition_y _cursorworldposition_z) (`KismetMathLibrary.BreakVector` (`self.CursorWorldPosition`)))
  (bind _gridsize (`self.GridSize`))
  (return (`KismetMathLibrary.MakeVector` (`/Game/RollOut/Libraries/FunctionLibrary.GridSnap` _cursorworldposition_x _gridsize) (`/Game/RollOut/Libraries/FunctionLibrary.GridSnap` _cursorworldposition_y _gridsize) (`/Game/RollOut/Libraries/FunctionLibrary.GridSnap` _cursorworldposition_z _gridsize))))

(fn `SlopeTrace`
  (params (TraceLocation :type "Vector Structure"))
  (returns (Difference :type "Float (double-precision)"))
  (bind (_returnvalue_x _returnvalue_y _returnvalue_z) (`KismetMathLibrary.BreakVector` (`self.K2_GetActorLocation`)))
  (bind _outhit (`KismetSystemLibrary.LineTraceSingle` (+ TraceLocation (0.0 0.0 1000.0)) (- TraceLocation (0.0 0.0 1000.0)) "TraceTypeQuery3"))
  (return (- _returnvalue_z (.z (`.ImpactPoint` (`GameplayStatics.BreakHitResult` _outhit))))))

(fn `UserConstructionScript`)