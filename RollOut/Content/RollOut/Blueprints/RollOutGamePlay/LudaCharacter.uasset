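; LudaCharacter is a character Blueprint for RollOut gameplay that sets up its camera view when play begins.
; BeginPlay activates the TopDown camera, centres it on world X/Y zero at its existing height, and deactivates FollowCam.
; When LudaMode is set, it then applies a one-time additive launch along world +Y, labelled as forward/backward rolling.
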(event `self.ReceiveBeginPlay`
  (bind _topdown (`self.TopDown`))
  ;[1 1 1] BeginPlay
  (`|ExecutionSequence`
    (:`then_0`
      (`ActorComponent.SetActive` _topdown true false)
      (`SceneComponent.K2_SetWorldLocation` _topdown (`KismetMathLibrary.MakeVector` 0.0 0.0 (.z (`SceneComponent.K2_GetComponentLocation` _topdown))) false false)
      (`ActorComponent.SetActive` (`self.FollowCam`) false false))
    (:`then_1`
      ;[1 1 1] Roll forwards/backwards
      (if (`self.LudaMode`)
        (`self.LaunchCharacter` (0.0 3000.0 0.0))))))

(fn `UserConstructionScript`)