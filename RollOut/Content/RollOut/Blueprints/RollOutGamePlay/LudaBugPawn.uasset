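; LudaBugPawn is a RollOut gameplay pawn that rolls its Luda component and starts in a top-down camera view.
; While LudaMode is on, Tick applies a frame-time-scaled impulse along world Y from RollTorque, using linear impulse rather than torque.
; BeginPlay activates the TopDown camera, centers it on the world origin at its existing height, and deactivates FollowCam.
; Nothing in these graphs sets LudaMode or RollTorque.
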(event `self.ReceiveTick`
  (params (DeltaSeconds :type "Float (single-precision)"))
  ;[1 1 1] Roll forwards/backwards
  (if (`self.LudaMode`)
    (`PrimitiveComponent.AddImpulse` (`self.Luda`) (`KismetMathLibrary.MakeVector` 0.0 (* DeltaSeconds (`self.RollTorque`))) "None" false)))

(event `self.ReceiveBeginPlay`
  (bind _topdown (`self.TopDown`))
  ;[1 1 1] BeginPlay
  (`ActorComponent.SetActive` _topdown true false)
  (`SceneComponent.K2_SetWorldLocation` _topdown (`KismetMathLibrary.MakeVector` 0.0 0.0 (.z (`SceneComponent.K2_GetComponentLocation` _topdown))) false false)
  (`ActorComponent.SetActive` (`self.FollowCam`) false false))

(fn `UserConstructionScript`)