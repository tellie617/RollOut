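; Player controller for the RollOut camera pawn that handles placing limited-quantity walls in build mode.
; On BeginPlay it spawns a construction manager and ghost wall, creates the HUD and caches pawn and PlayerState references.
; While building, Tick moves the ghost to the cursor, with trace distance extended by spring-arm length.
; Releasing Drop checks overlap and stock, queues construction, decrements that wall type's count and kills the ghost.
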(event `self.ReceiveBeginPlay`
  (bind _returnvalue (`KismetMathLibrary.MakeTransform` (0.0 0.0 0.0)))
  ;[1 1 1] BeginPlay
  (`|ExecutionSequence`
    (:`then_0`
      (`self.ReferenceCasts`))
    (:`then_1`
      (bind _returnvalue_2 (`|SpawnActorFromClass` "/Game/RollOut/Blueprints/Construction/ConstructionManagerBP.ConstructionManagerBP_C" _returnvalue "AlwaysSpawn" "OverrideRootScale"))
      (set `self.ConstructionManagerRef` _returnvalue_2))
    (:`then_2`
      (bind _returnvalue_3 (`|SpawnActorFromClass` "/Game/RollOut/Blueprints/Walls/MasterBPs/GhostWalBP.GhostWalBP_C" _returnvalue "AlwaysSpawn" "OverrideRootScale" null self))
      (set `self.GhostBuildingRef` _returnvalue_3))
    (:`then_3`
      (`WidgetBlueprintLibrary.SetInputMode_GameAndUIEx` self null "LockAlways" false)
      (`self.CreateHUD`)
      (`UserWidget.AddToViewport` (`self.MainHUDRef`) 0))
    (:`then_4`
      (bind _asroll_out_player_state (cast `/Game/RollOut/Blueprints/RollOutGamePlay/RollOutPlayerState` (`self.PlayerState`)))
      (set `self.PlayerStateReference` _asroll_out_player_state))))

(event `self.ReceiveTick`
  (params (DeltaSeconds :type "Float (single-precision)"))
  ;[1 1 1] EventTick
  (if (`self.BuildModeActive`)
    (if (!= (`self.GhostBuildingRef`) null)
      (`/Game/RollOut/Blueprints/Walls/MasterBPs/GhostWalBP.SetCursorPosition` (`self.GhostBuildingRef`) (`/Game/RollOut/Libraries/FunctionLibrary.SetCursorWorldPosition` self (`self.SetSightDistance`))))))

(event `InputAction|Drop`
  (params (Key :type "Key Structure" :default "AnyKey"))
  ;[1 1 1] Drop
  (:`Released`
    (bind _bool (`self.CheckQty`))
    (if (and (`self.BuildModeActive`) (not (`/Game/RollOut/Blueprints/Walls/MasterBPs/GhostWalBP.GetIsOverlapping` (`self.GhostBuildingRef`))) _bool)
      (bind _constructionstruct (`/Game/RollOut/Blueprints/Walls/MasterBPs/GhostWalBP.GetConstructionStruct` (`self.GhostBuildingRef`)))
      (`/Game/RollOut/Blueprints/Construction/ConstructionManagerBP.QueueConstruction` (`self.ConstructionManagerRef`) _constructionstruct)
      (`self.RemoveQty`)
      (`/Game/RollOut/Blueprints/Walls/MasterBPs/GhostWalBP.KillGhost` (`self.GhostBuildingRef`))
      (set `/Game/RollOut/Blueprints/HUD/MainUI_HUD.WallConstructed` true (`self.MainHUDRef`)))))

(fn `CheckQty`
  (returns (Bool :type Boolean))
  (locals (Qty :type Integer))
  (bind _ghostbuildingref (`self.GhostBuildingRef`))
  ;[1 1 1] Check Quantity
  (if (== (`/Game/RollOut/Blueprints/Walls/MasterBPs/GhostWalBP.WallClass` _ghostbuildingref) "/Game/RollOut/Blueprints/Walls/Angle/AngledWallChildBP.AngledWallChildBP_C")
    (set `local.Qty` (`/Game/RollOut/Blueprints/RollOutGamePlay/RollOutPlayerState.AngledQty` (`self.PlayerStateReference`)))
    (return (> (`local.Qty`) 0))
    (elif (== (`/Game/RollOut/Blueprints/Walls/MasterBPs/GhostWalBP.WallClass` _ghostbuildingref) "/Game/RollOut/Blueprints/Walls/Crumble/CrumbleWallChildBP.CrumbleWallChildBP_C")
      (set `local.Qty` (`/Game/RollOut/Blueprints/RollOutGamePlay/RollOutPlayerState.CrumbleQty` (`self.PlayerStateReference`)))
      (return (> (`local.Qty`) 0))
      (elif (== (`/Game/RollOut/Blueprints/Walls/MasterBPs/GhostWalBP.WallClass` _ghostbuildingref) "/Game/RollOut/Blueprints/Walls/Ramp/RampWallChildBP.RampWallChildBP_C")
        (set `local.Qty` (`/Game/RollOut/Blueprints/RollOutGamePlay/RollOutPlayerState.RampQty` (`self.PlayerStateReference`)))
        (return (> (`local.Qty`) 0))
        (elif (== (`/Game/RollOut/Blueprints/Walls/MasterBPs/GhostWalBP.WallClass` _ghostbuildingref) "/Game/RollOut/Blueprints/Walls/Bounce/BounceWallChildBP.BounceWallChildBP_C")
          (set `local.Qty` (`/Game/RollOut/Blueprints/RollOutGamePlay/RollOutPlayerState.BounceQty` (`self.PlayerStateReference`)))
          (return (> (`local.Qty`) 0))
          (else
            (set `local.Qty` 0)))))))

(fn `CheckWallType`
  (returns (WallType :type String))
  (locals (Output :type String))
  (bind _ghostbuildingref (`self.GhostBuildingRef`))
  (if (== (`/Game/RollOut/Blueprints/Walls/MasterBPs/GhostWalBP.WallClass` _ghostbuildingref) "/Game/RollOut/Blueprints/Walls/Angle/AngledWallChildBP.AngledWallChildBP_C")
    (set `local.Output` "angled")
    (return (`local.Output`))
    (elif (== (`/Game/RollOut/Blueprints/Walls/MasterBPs/GhostWalBP.WallClass` _ghostbuildingref) "/Game/RollOut/Blueprints/Walls/Crumble/CrumbleWallChildBP.CrumbleWallChildBP_C")
      (set `local.Output` "crumble")
      (return (`local.Output`))
      (elif (== (`/Game/RollOut/Blueprints/Walls/MasterBPs/GhostWalBP.WallClass` _ghostbuildingref) "/Game/RollOut/Blueprints/Walls/Ramp/RampWallChildBP.RampWallChildBP_C")
        (set `local.Output` "ramp")
        (return (`local.Output`))
        (elif (== (`/Game/RollOut/Blueprints/Walls/MasterBPs/GhostWalBP.WallClass` _ghostbuildingref) "/Game/RollOut/Blueprints/Walls/Bounce/BounceWallChildBP.BounceWallChildBP_C")
          (set `local.Output` "bounce")
          (return (`local.Output`))
          (else
            (set `local.Output` "")))))))

(fn `MovementSpeedCalculation`
  (returns (MoveSensitivity :type "Float (double-precision)"))
  (return (`KismetMathLibrary.FClamp` (/ (`SpringArmComponent.TargetArmLength` (`/Game/RollOut/Blueprints/RollOutGamePlay/RollOutCameraPawn.SpringArm` (`self.CameraPawnRef`))) 100.0) 5.0 20.0)))

(fn `RemoveQty`
  (locals (temp :type Integer))
  (bind _playerstatereference (`self.PlayerStateReference`))
  ;[1 1 1] RemoveQuantiry
  (bind _walltype (`self.CheckWallType`))
  (switch `string` _walltype
    (:`Default`
      (return))
    (:`angled`
      (bind _result (`/Engine/EditorBlueprintResources/StandardMacros.DecrementInt` (`/Game/RollOut/Blueprints/RollOutGamePlay/RollOutPlayerState.AngledQty` _playerstatereference))
        (:`  `
          (`KismetSystemLibrary.PrintText` (`KismetTextLibrary.Conv_IntToText` _result))
          (return))))
    (:`crumble`
      (bind _result_2 (`/Engine/EditorBlueprintResources/StandardMacros.DecrementInt` (`/Game/RollOut/Blueprints/RollOutGamePlay/RollOutPlayerState.CrumbleQty` _playerstatereference))
        (:`  `
          (`KismetSystemLibrary.PrintText` (`KismetTextLibrary.Conv_IntToText` _result_2)))))
    (:`ramp`
      (`/Engine/EditorBlueprintResources/StandardMacros.DecrementInt` (`/Game/RollOut/Blueprints/RollOutGamePlay/RollOutPlayerState.RampQty` _playerstatereference)
        (:`  `
          (return))))
    (:`bounce`
      (`/Engine/EditorBlueprintResources/StandardMacros.DecrementInt` (`/Game/RollOut/Blueprints/RollOutGamePlay/RollOutPlayerState.BounceQty` _playerstatereference)
        (:`  `
          (return))))))

(fn `SetSightDistance`
  (returns (SightDistance :type "Float (double-precision)"))
  (return (+ (`self.SightDistance`) (`SpringArmComponent.TargetArmLength` (`/Game/RollOut/Blueprints/RollOutGamePlay/RollOutCameraPawn.SpringArm` (`self.CameraPawnRef`))))))

(fn `UserConstructionScript`)